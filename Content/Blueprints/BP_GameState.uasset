(event `self.OnVictory`
  (for _array_element (`self.PlayerArray`)
    (bind _asnet_player_state (cast `NetPlayerState` _array_element))
    (bind (_data_nickname _data_customizationdata _data_teamid) (break `SPlayerInfo` (`NetPlayerState.Data` _asnet_player_state)))
    (switch `EPlayerTeam` _data_teamid
      (:`TEAM_Blue`
        (bind _asbp_avatar (cast `/Game/Blueprints/BP_Avatar` (`PlayerState.PawnPrivate` _asnet_player_state) :!pure true))
        (`/Game/Blueprints/BP_Avatar.OnPlayerLost` _asbp_avatar))
      (:`TEAM_Red`
        (`/Game/Blueprints/BP_Avatar.OnPlayerWin` _asbp_avatar))))
  (`self.ShowMessage`))

(event `self.OnRestart`
  (`Widget.RemoveFromParent` (`self.Message Widget`)))

(fn `ShowMessage`
  (bind _returnvalue (`self.GetPlayerStateByIndex` (`self.WinningPlayer`)))
  (bind _returnvalue_2 (`|CreateWidget` "/Game/Blueprints/UMG/W_GameResults.W_GameResults_C" null (`KismetMathLibrary.SelectText` (`|FormatText` "{Name} Wins!" (`.NickName` (break `SPlayerInfo` (`NetPlayerState.Data` _returnvalue)))) "You Lose!" (`|EnumEquality` (`.TeamID` (break `SPlayerInfo` (`NetPlayerState.Data` (cast `NetPlayerState` (`Controller.PlayerState` (`GameplayStatics.GetPlayerController` 0)) :!pure true)))) "TEAM_Blue"))))
  (set `self.Message Widget` _returnvalue_2)
  (`UserWidget.AddToViewport` _returnvalue_2 0))

(fn `UserConstructionScript`)